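; bhScale is a short-lived actor that shrinks an overlapping Enemy-tagged actor toward zero scale.
; Tick, throttled by a short Delay, raises Alpha and lerps the actor's current scale toward zero, so shrinking compounds.
; The target comes straight from the overlap event's OtherActor pin, as that event runs no logic.
; Five seconds after BeginPlay, it destroys itself, then calls destroy on that OtherActor without a tag check.
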(event EventBeginPlay
  (Utilities|FlowControl|Delay 0 5.0)
  (Actor|DestroyActor)
  (Actor|DestroyActor (stale EventActorBeginOverlap OtherActor)))

(event EventActorBeginOverlap
  (params (OtherActor :type Actor%20Object%20Reference)))

(event EventTick
  (params (DeltaSeconds :type Float%20%28single-precision%29))
  (Utilities|FlowControl|Delay 0 0.05)
  (if (Utilities|Array|ContainsItem (Variables|/Script/Engine.Actor|GetTags (stale EventActorBeginOverlap OtherActor)) "Enemy")
    (Variables|Default|Setalpha (+ (Variables|Default|Getalpha) 0.05))
    (Transformation|SetActorScale3D (stale EventActorBeginOverlap OtherActor) (Math|Vector|Lerp(Vector) (.Scale (Math|Transform|BreakTransform (Transformation|GetActorTransform (stale EventActorBeginOverlap OtherActor)))) "0, 0, 0" (Variables|Default|Getalpha)))))

(fn ConstructionScript)