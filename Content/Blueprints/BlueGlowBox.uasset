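; BlueGlowBox is an actor that reacts to projectile hits only while the player stands in blue light.
; It caches the first MyCharacter on BeginPlay, then on a hit by MyProjectile checks that character's InBlueLight flag.
; When the flag is set, it spawns an explosion at the hit location and tells its Spawner to display an object.
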(event EventBeginPlay
  (bind _outactors (Actor|GetAllActorsOfClass "/Game/Blueprints/MyCharacter.MyCharacter_C"))
  (bind _asmycharacter_c (Utilities|Casting|CastToMyCharacter (Utilities|Array|Get(acopy) _outactors)))
  (Variables|Default|SetPlayer%20Reference _asmycharacter_c))

(event EventHit
  (params (MyComp :type Primitive%20Component%20Object%20Reference) (Other :type Actor%20Object%20Reference) (OtherComp :type Primitive%20Component%20Object%20Reference) (bSelfMoved :type Boolean) (HitLocation :type Vector :default "0, 0, 0") (HitNormal :type Vector :default "0, 0, 0") (NormalImpulse :type Vector :default "0, 0, 0") (Hit :type Hit%20Result%20Structure%20%28by%20ref%29))
  (Utilities|Casting|CastToMyProjectile Other)
  (if (Variables|/Game/Blueprints/MyCharacter.MyCharacter_C|GetInBlueLight (Variables|Default|GetPlayer%20Reference))
    (Effects|SpawnEmitteratLocation "/Game/Particles/P_Explosion.P_Explosion" HitLocation)
    (Default|DisplayObject (Variables|Default|GetSpawner))))

(fn ConstructionScript)