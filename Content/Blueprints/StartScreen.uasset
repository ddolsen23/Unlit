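; HUD Blueprint for the start screen, drawing a title, divider, tagline and press-to-start prompt on the canvas.
; Each DrawHUD centers the text horizontally using measured sizes, at set fractions of screen height.
; A delta-time counter with a direction flag ping-pongs the prompt's alpha to make it pulse.
; Pressing B starts streaming in Dungeon_Start without blocking or making it visible.
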(event EventDrawHUD
  (params (SizeX :type Integer) (SizeY :type Integer))
  (bind _returnvalue (Utilities|Time|GetWorldDeltaSeconds))
  (bind _presstostartsize (Variables|Default|GetPressToStartSize))
  (bind _presstostart (Variables|Default|GetPressToStart))
  (bind _dividersize (Variables|Default|GetDividerSize))
  (bind _title (Variables|Default|GetTitle))
  (bind _titlesize (Variables|Default|GetTitleSize))
  (bind _divider (Variables|Default|GetDivider))
  (bind _enterthedarksize (Variables|Default|GetEnterTheDarkSize))
  (bind _enterthedarkness (Variables|Default|GetEnterTheDarkness))
  (bind _alphablenddur (Variables|Default|GetAlphaBlendDur))
  (bind (_outwidth _outheight) (Class|HUD|GetTextSize _divider "/Game/Fonts/SegueUI.SegueUI" _dividersize))
  (bind (_outwidth_2 _outheight_2) (Class|HUD|GetTextSize _presstostart "/Game/Fonts/SegueUI.SegueUI" _presstostartsize))
  (bind (_outwidth_3 _outheight_3) (Class|HUD|GetTextSize _title "/Game/Fonts/SegueUI.SegueUI" _titlesize))
  (bind (_outwidth_4 _outheight_4) (Class|HUD|GetTextSize _enterthedarkness "/Game/Fonts/SegueUI.SegueUI" _enterthedarksize))
  (HUD|DrawText _title "(R=0.865000,G=0.865000,B=0.865000,A=1.000000)" (- (* SizeX 0.5) (/ _outwidth_3 2.0)) (- (* SizeY 0.35) (/ _outheight_3 2.0)) "/Game/Fonts/SegueUI.SegueUI" _titlesize false)
  (if (or (Math|Boolean|Equal(Boolean) (> (Variables|Default|GetAlphaBlendTime) _alphablenddur) true) (Math|Boolean|Equal(Boolean) (Variables|Default|Getalphapos) false))
    (Variables|Default|SetAlphaBlendTime (- (Variables|Default|GetAlphaBlendTime) _returnvalue))
    (Variables|Default|Setalphapos (<= (Variables|Default|GetAlphaBlendTime) 0.0))
    (else
      (Variables|Default|SetAlphaBlendTime (+ _returnvalue (Variables|Default|GetAlphaBlendTime)))
      (Variables|Default|Setalphapos true)))
  (HUD|DrawText _presstostart (Utilities|Struct|MakeLinearColor 255.0 255.0 255.0 (/ (Variables|Default|GetAlphaBlendTime) _alphablenddur)) (- (* SizeX 0.5) (/ _outwidth_2 2.0)) (- (* SizeY 0.62) (/ _outheight_2 2.0)) "/Game/Fonts/SegueUI.SegueUI" _presstostartsize false)
  (HUD|DrawText _divider "(R=0.955000,G=0.955000,B=0.955000,A=1.000000)" (- (* SizeX 0.5) (/ _outwidth 2.0)) (- (* SizeY 0.45) (/ _outheight 2.0)) "/Game/Fonts/SegueUI.SegueUI" _dividersize false)
  (HUD|DrawText _enterthedarkness "(R=0.955000,G=0.955000,B=0.955000,A=1.000000)" (- (* SizeX 0.5) (/ _outwidth_4 2.0)) (- (* SizeY 0.55) (/ _outheight_4 2.0)) "/Game/Fonts/SegueUI.SegueUI" _enterthedarksize false))

(event Input|KeyboardEvents|B
  (:Pressed
    (Game|LoadStreamLevel(byName) "Dungeon_Start" false)))

(fn ConstructionScript)