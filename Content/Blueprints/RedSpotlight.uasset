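; RedSpotlight is a spotlight actor that notifies MyCharacter when it enters or leaves the light's area.
; On BeginPlay, StartVisible sets the spotlight's visibility and switches StaticMesh1 between query-and-physics collision and none.
; Actor begin and end overlaps cast the other actor to MyCharacter and call EnterRedSpotlight or ExitRedSpotlight, leaving the response to the character.
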(event EventActorBeginOverlap
  (params (OtherActor :type Actor%20Object%20Reference))
  (bind _asmycharacter_c (Utilities|Casting|CastToMyCharacter OtherActor))
  (Default|EnterRedSpotlight _asmycharacter_c))

(event EventActorEndOverlap
  (params (OtherActor :type Actor%20Object%20Reference))
  (bind _asmycharacter_c (Utilities|Casting|CastToMyCharacter OtherActor))
  (Default|ExitRedSpotlight _asmycharacter_c))

(event EventBeginPlay
  (bind _start_visible (Variables|Default|GetStart_Visible))
  (bind _staticmesh1 (Variables|Default|GetStaticMesh1))
  (Rendering|SetVisibility (Variables|Default|GetSpotLight1) _start_visible false)
  (if _start_visible
    (Collision|SetCollisionEnabled _staticmesh1 "QueryAndPhysics")
    (else
      (Collision|SetCollisionEnabled _staticmesh1 "NoCollision"))))

(fn ConstructionScript)