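; Red box spawner actor that makes a glow box exist only while the player character is in red light, and can toggle a set of walls.
; Tick polls the player's InRedLight flag, spawning a RedGlowBox at its own transform or destroying it.
; Each box receives a back-reference to its spawner.
; ToggleWalls flips visibility and collision on the assigned walls together, with initial state read from the first wall.
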(event EventTick
  (params (DeltaSeconds :type Float%20%28single-precision%29))
  (if (and (Variables|/Game/Blueprints/MyCharacter.MyCharacter_C|GetInRedLight (Variables|Default|GetPlayer%20Reference)) (not (Variables|Default|GetVisible)))
    (bind _returnvalue (Game|SpawnActorfromClass "/Game/Blueprints/RedGlowBox.RedGlowBox_C" (Transformation|GetActorTransform) true 0))
    (Variables|Default|SetBox _returnvalue)
    (Variables|Default|SetVisible true)
    (Variables|/Game/Blueprints/RedGlowBox.RedGlowBox_C|SetSpawner (Variables|Default|GetBox) self)
    (elif (and (not (Variables|/Game/Blueprints/MyCharacter.MyCharacter_C|GetInRedLight (Variables|Default|GetPlayer%20Reference))) (Variables|Default|GetVisible))
      (Actor|DestroyActor (Variables|Default|GetBox))
      (Variables|Default|SetVisible false))))

(event EventBeginPlay
  (bind _outactors (Actor|GetAllActorsOfClass "/Game/Blueprints/MyCharacter.MyCharacter_C"))
  (bind _asmycharacter_c (Utilities|Casting|CastToMyCharacter (Utilities|Array|Get(acopy) _outactors)))
  (Variables|Default|SetPlayer%20Reference _asmycharacter_c)
  (Variables|Default|SetWallsOn (Variables|/Game/Architecture/RedShieldWall.RedShieldWall_C|GetStart_Visible (Utilities|Array|Get(acopy) (Variables|Default|GetWalls)))))

(fn ConstructionScript)

(fn ToggleWalls
  (if (Variables|Default|GetWallsOn)
    (for _index (range 0 (Utilities|Array|Length (Variables|Default|GetWalls)))
      (Rendering|SetVisibility (VehicleSound|GetRootComponent (Utilities|Array|Get(acopy) (Variables|Default|GetWalls) _index)) false true)
      (Collision|SetCollisionEnabled (Variables|/Game/Architecture/RedShieldWall.RedShieldWall_C|GetWall_400x200_0 (Utilities|Array|Get(acopy) (Variables|Default|GetWalls) _index)) "NoCollision"))
    (Variables|Default|SetWallsOn false)
    (else
      (for _index_2 (range 0 (Utilities|Array|Length (Variables|Default|GetWalls)))
        (Rendering|SetVisibility (VehicleSound|GetRootComponent (Utilities|Array|Get(acopy) (Variables|Default|GetWalls) _index_2)) true true)
        (Collision|SetCollisionEnabled (Variables|/Game/Architecture/RedShieldWall.RedShieldWall_C|GetWall_400x200_0 (Utilities|Array|Get(acopy) (Variables|Default|GetWalls) _index_2)) "QueryAndPhysics"))
      (Variables|Default|SetWallsOn true))))