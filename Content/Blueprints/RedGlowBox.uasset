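; RedGlowBox is a target that toggles walls when struck by a red-glowing projectile.
; On hit, it casts the other actor to MyProjectile and checks its GlowLight color for strong red with low green and blue.
; A match plays an alert tone, spawns an explosion at the hit location and calls ToggleWalls on its Spawner.
; BeginPlay caches the first MyCharacter as PlayerReference, which the hit logic does not use.
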(event EventBeginPlay
  (bind _outactors (Actor|GetAllActorsOfClass "/Game/Blueprints/MyCharacter.MyCharacter_C"))
  (bind _asmycharacter_c (Utilities|Casting|CastToMyCharacter (Utilities|Array|Get(acopy) _outactors)))
  (Variables|Default|SetPlayer%20Reference _asmycharacter_c))

(event EventHit
  (params (MyComp :type Primitive%20Component%20Object%20Reference) (Other :type Actor%20Object%20Reference) (OtherComp :type Primitive%20Component%20Object%20Reference) (bSelfMoved :type Boolean) (HitLocation :type Vector :default "0, 0, 0") (HitNormal :type Vector :default "0, 0, 0") (NormalImpulse :type Vector :default "0, 0, 0") (Hit :type Hit%20Result%20Structure%20%28by%20ref%29))
  (bind _asmyprojectile_c (Utilities|Casting|CastToMyProjectile Other))
  (if (Math|Boolean|ANDBoolean (> (.R (Math|Color|BreakColor (Variables|/Script/Engine.LightComponentBase|GetLightColor (Variables|/Game/Blueprints/MyProjectile.MyProjectile_C|GetGlowLight _asmyprojectile_c)))) 100) (< (.G (Math|Color|BreakColor (Variables|/Script/Engine.LightComponentBase|GetLightColor (Variables|/Game/Blueprints/MyProjectile.MyProjectile_C|GetGlowLight _asmyprojectile_c)))) 20) (< (.B (Math|Color|BreakColor (Variables|/Script/Engine.LightComponentBase|GetLightColor (Variables|/Game/Blueprints/MyProjectile.MyProjectile_C|GetGlowLight _asmyprojectile_c)))) 20))
    (if (Math|Boolean|ANDBoolean (> (.R (Math|Color|BreakColor (Variables|/Script/Engine.LightComponentBase|GetLightColor (Variables|/Game/Blueprints/MyProjectile.MyProjectile_C|GetGlowLight _asmyprojectile_c)))) 100) (< (.G (Math|Color|BreakColor (Variables|/Script/Engine.LightComponentBase|GetLightColor (Variables|/Game/Blueprints/MyProjectile.MyProjectile_C|GetGlowLight _asmyprojectile_c)))) 20) (< (.B (Math|Color|BreakColor (Variables|/Script/Engine.LightComponentBase|GetLightColor (Variables|/Game/Blueprints/MyProjectile.MyProjectile_C|GetGlowLight _asmyprojectile_c)))) 20))
      (Audio|PlaySoundatLocation "/Game/Audio/alert_tone.alert_tone" "0, 0, 0" 0.15 0.75))
    (Effects|SpawnEmitteratLocation "/Game/Particles/P_Explosion.P_Explosion" HitLocation)
    (Default|ToggleWalls (Variables|Default|GetSpawner))))

(fn ConstructionScript)