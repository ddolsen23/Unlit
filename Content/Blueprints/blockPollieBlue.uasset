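; Blue block actor that slides horizontally when hit by a MyProjectile, provided its material is not OrangeGlow and the player is in blue light but not red.
; The overlap starts a delayed move, which divides the XY offset toward the overlapping actor's location into equal steps.
; A looping follow timer applies the steps with swept moves, reverts failed ones, and clears itself when the step count runs out.
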(event Custom|follow
  (bind _add (Variables|Default|Getadd))
  (bind (_x _y) (Math|Vector|BreakVector _add))
  (Variables|Default|SetprevLocation (Variables|Default|GetmyLocation))
  (bind _returnvalue (Transformation|SetActorLocation self (+ (Variables|Default|GetmyLocation) (Math|Vector|MakeVector _x _y 0.0)) true))
  (if _returnvalue
    _
    (else
      (Transformation|SetActorLocation (Variables|Default|GetprevLocation) false)))
  (Variables|Default|SetmyLocation (+ (Variables|Default|GetmyLocation) (Math|Vector|MakeVector _x _y 0.0)))
  (Variables|Default|Setdistance (- (Variables|Default|Getdistance) 1.0))
  (if (not (> (Variables|Default|Getdistance) 0.0))
    (Utilities|Time|ClearTimerbyFunctionName 0 "follow")))

(event Custom|move
  (bind _self self)
  (bind _returnvalue (Transformation|GetActorLocation _self))
  (Utilities|Time|ClearTimerbyFunctionName 0 "move")
  (Variables|Default|SetmyLocation _returnvalue)
  (Variables|Default|SetotherLocation (Math|Vector|MakeVector (- (.X (Math|Vector|BreakVector (Transformation|GetActorLocation (stale EventActorBeginOverlap OtherActor)))) 0.0) (- (.Y (Math|Vector|BreakVector (Transformation|GetActorLocation (stale EventActorBeginOverlap OtherActor)))) 0.0) 0.0))
  (Variables|Default|SetprevLocation _returnvalue)
  (Variables|Default|Setadd (/ (- (Variables|Default|GetotherLocation) (Variables|Default|GetmyLocation)) "30.000000,30.000000,30.000000"))
  (Variables|Default|Setdistance 3e+01)
  (Utilities|Time|SetTimerbyFunctionName 0 "follow" 0.04 true))

(event EventActorBeginOverlap
  (params (OtherActor :type Actor%20Object%20Reference))
  (bind _playerref (Variables|Default|GetplayerRef))
  (if (== "/Game/Blueprints/MyProjectile.MyProjectile_C" (Utilities|GetClass OtherActor))
    (if (not (Utilities|Enum|Equal(Enum) (Utilities|String|MakeLiteralString "OrangeGlow") (Utilities|String|ToString(Object) (Rendering|Material|GetMaterial (Variables|Default|GetblockPollie) 0))))
      (if (not (Variables|/Game/Blueprints/MyCharacter.MyCharacter_C|GetInRedLight _playerref))
        (if (Variables|/Game/Blueprints/MyCharacter.MyCharacter_C|GetInBlueLight _playerref)
          (Utilities|Time|SetTimerbyFunctionName 0 "move" 1.5))))))

(event EventBeginPlay
  (bind _outactors (Actor|GetAllActorsOfClass "/Game/Blueprints/MyCharacter.MyCharacter_C"))
  (bind _asmycharacter_c (Utilities|Casting|CastToMyCharacter (Utilities|Array|Get(acopy) _outactors)))
  (Variables|Default|SetplayerRef _asmycharacter_c))

(fn ConstructionScript)