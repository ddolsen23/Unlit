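; Spawner actor that shows a BlueGlowBox at its transform while the player is in blue light and can turn on a hidden object.
; Tick polls the player's InBlueLight flag, spawning the box with a back-reference to itself and destroying it when the light leaves.
; DisplayObject latches TurnedOn so the box persists, zeroes its light, then shows AppearObject and enables collision on its root or child static meshes.
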(event EventTick
  (params (DeltaSeconds :type Float%20%28single-precision%29))
  (if (and (Variables|/Game/Blueprints/MyCharacter.MyCharacter_C|GetInBlueLight (Variables|Default|GetPlayer%20Reference)) (not (Variables|Default|GetVisible)))
    (bind _returnvalue (Game|SpawnActorfromClass "/Game/Blueprints/BlueGlowBox.BlueGlowBox_C" (Transformation|GetActorTransform) true 0))
    (Variables|Default|SetBox _returnvalue)
    (Variables|Default|SetVisible true)
    (Variables|/Game/Blueprints/BlueGlowBox.BlueGlowBox_C|SetSpawner (Variables|Default|GetBox) self)
    (elif (Math|Boolean|ANDBoolean (not (Variables|/Game/Blueprints/MyCharacter.MyCharacter_C|GetInBlueLight (Variables|Default|GetPlayer%20Reference))) (Variables|Default|GetVisible) (not (Variables|Default|GetTurnedOn)))
      (Actor|DestroyActor (Variables|Default|GetBox))
      (Variables|Default|SetVisible false))))

(event EventBeginPlay
  (bind _outactors (Actor|GetAllActorsOfClass 0 "/Game/Blueprints/MyCharacter.MyCharacter_C"))
  (bind _asmycharacter_c (Utilities|Casting|CastToMyCharacter (Utilities|Array|Get(acopy) _outactors)))
  (Variables|Default|SetPlayer%20Reference _asmycharacter_c))

(fn ConstructionScript)

(fn DisplayObject
  (bind _appear_object (Variables|Default|GetAppear_Object))
  (bind _returnvalue (VehicleSound|GetRootComponent _appear_object))
  (Variables|Default|SetTurnedOn true)
  (Rendering|Components|Light|SetIntensity (Variables|/Game/Blueprints/BlueGlowBox.BlueGlowBox_C|GetPointLight1 (Variables|Default|GetBox)) 0.0)
  (Rendering|SetVisibility _returnvalue true true)
  (bind _asstaticmeshcomponent (Utilities|Casting|CastToStaticMeshComponent _returnvalue)
    (:then
      (Collision|SetCollisionEnabled _asstaticmeshcomponent "QueryAndPhysics"))
    (:CastFailed
      (for _array_element (Components|GetChildrenComponents _returnvalue true)
        (bind _asstaticmeshcomponent_2 (Utilities|Casting|CastToStaticMeshComponent _array_element))
        (Collision|SetCollisionEnabled _asstaticmeshcomponent_2 "QueryAndPhysics")))))